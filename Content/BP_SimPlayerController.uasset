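; Player controller for a tribe and settlement simulation map, handling click selection and the UI that shows what was selected.
; BeginPlay creates the heatmap menu and a hidden info panel.
; Left clicks call HandleMapClick; tribe and settlement selection events fill and show that shared panel, printing a Czech debug message.
; Cell selection hides it and spawns a detail widget given the cursor's hit location, which HideAllPanels removes.
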(event EventBeginPlay
  (bind _returnvalue (UserInterface|CreateWidget "/Game/WBP_InfoPanel.WBP_InfoPanel_C"))
  (Variables|Default|SetInfoWidgetRef _returnvalue)
  (UserInterface|Viewport|AddtoViewport (Variables|Default|GetInfoWidgetRef) 0)
  (Widget|SetVisibility (Variables|Default|GetInfoWidgetRef) "Hidden")
  (bind _returnvalue_2 (UserInterface|CreateWidget "/Game/WBP_HeatmapMenu.WBP_HeatmapMenu_C"))
  (UserInterface|Viewport|AddtoViewport _returnvalue_2 0))

(event EventTick
  (params (DeltaSeconds :type Float%20%28single-precision%29)))

(event EventOnTribeSelected
  (params (TribeData :type Tribe%20Data%20Structure))
  (bind _infowidgetref (Variables|Default|GetInfoWidgetRef))
  (Default|UpdateTribeInfo _infowidgetref (Utilities|Struct|MakeTribeData (.tribeid TribeData) (.position TribeData) (.population TribeData) (.state TribeData) (.campdaysremaining TribeData) (.campscore TribeData) (.interactioncooldowndays TribeData) (.inventory TribeData) (.knowledge TribeData) (.culture TribeData) (.targetregion TribeData) (.nextstrategicdecisionday TribeData) (.tribecolor TribeData) (.daysatcamp TribeData) (.bfollowingherd TribeData) (.bhasforcedtarget TribeData) (.forcedtarget TribeData) "(X=0.000000,Y=0.000000)" "(X=0.000000,Y=0.000000)" 0.0))
  (Widget|SetVisibility _infowidgetref "Visible")
  (Development|PrintString "Kliknuto na kmen"))

(event EventOnSettlementSelected
  (params (SettlementData :type Settlement%20Data%20Structure))
  (bind _infowidgetref (Variables|Default|GetInfoWidgetRef))
  (Default|UpdateSettlementInfo _infowidgetref (Utilities|Struct|MakeSettlementData (.settlementid SettlementData) (.nationid SettlementData) (.position SettlementData) (.population SettlementData) (.interactioncooldowndays SettlementData) (.inventory SettlementData) (.color SettlementData) (.gatherradius SettlementData) (.splitcount SettlementData) (.knowledge SettlementData) (.culture SettlementData) (.localfoodpotential SettlementData) (.localwoodpotential SettlementData) (.localwaterpotential SettlementData) (.localstonepotential SettlementData) (.resourcepressure SettlementData) (.ecologicalpressure SettlementData) (.bhasforcedexpansion SettlementData) (.forcedexpansiontarget SettlementData) 0.0))
  (Widget|SetVisibility _infowidgetref "Visible")
  (Development|PrintString "Kliknuto na osadu"))

(event EventOnCellSelected
  (params (StaticCellData :type Cell%20Static%20Data%20Structure) (DynamicCellData :type Cell%20Dynamic%20Data%20Structure))
  (Widget|SetVisibility (Variables|Default|GetInfoWidgetRef) "Hidden")
  (bind _returnvalue (UserInterface|CreateWidget "/Game/WBP_CellDetail.WBP_CellDetail_C"))
  (Variables|Default|SetActiveCellWidget _returnvalue)
  (bind _output_get (Variables|Default|SetHit%20Result%20Location (.location (.HitResult (Game|Player|GetHitResultUnderCursorbyChannel "TraceTypeQuery1" true)))))
  (Default|InitCellData (Variables|Default|GetActiveCellWidget) _output_get StaticCellData DynamicCellData)
  (UserInterface|Viewport|AddtoViewport (Variables|Default|GetActiveCellWidget) 0))

(event EventHideAllPanels
  (bind _activecellwidget (Variables|Default|GetActiveCellWidget))
  (Utilities|IsValid _activecellwidget
    (:Is%20Valid
      (Widget|RemovefromParent _activecellwidget))))

(event Input|MouseEvents|LeftMouseButton
  (params (Key :type Key%20Structure :default "None"))
  (:Pressed
    (Class|SimPlayerController|HandleMapClick)))

(fn ConstructionScript)